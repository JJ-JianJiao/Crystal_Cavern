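; Player pawn moved by physics torque on its static mesh, with a spring arm.
; Both movement axes feed one torque node, scaled by direction and acceleration variables, and the camera fades in on BeginPlay.
; Any damage triggers a one-shot restart that fades the camera out, waits, then reopens the current level.
; Helper functions set uniform actor scale and spring arm length, pitch and yaw.
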(event `self.ReceiveBeginPlay`
  ;[1 1 1] Start Level Camera Fade
  (`PlayerCameraManager.StartCameraFade` :`self` (`GameplayStatics.GetPlayerCameraManager` 0) :`FromAlpha` 1.0 :`Duration` 3.0))

(event `InputAxis|Move Forward/Backwards`
  (params (AxisValue :type "Float (single-precision)"))
  (bind _acceleration_multiplier (`self.Acceleration multiplier`))
  ;[1 1 1] Player Pawn Movement
  (`PrimitiveComponent.AddTorqueInRadians` (`self.StaticMesh`) (`KismetMathLibrary.MakeVector` (* (stale `InputAxis|Move Left/Right` AxisValue) (* (`self.Left Right Direction`) _acceleration_multiplier)) (* AxisValue (* (`self.Forward Backward Direction`) _acceleration_multiplier))) "None" true :!label _label))

(event `InputAxis|Move Left/Right`
  (params (AxisValue :type "Float (single-precision)"))
  ;[1 1 1] Player Pawn Movement
  (goto _label))

(event `self.ReceiveAnyDamage`
  (params (Damage :type "Float (single-precision)") (DamageType :type "DamageType Object Reference") (InstigatedBy :type "Controller Object Reference") (DamageCauser :type "Actor Object Reference"))
  ;[1 1 1] Get Damage and Restart game
  (`self.Restart Level`))

(fn `Adjust Spring Arm`
  (params (Pitch :type "Float (double-precision)") (Distance :type "Float (double-precision)") (Yaw :type "Float (double-precision)"))
  (bind _springarm (`self.SpringArm`))
  (set `SpringArmComponent.TargetArmLength` Distance _springarm)
  (`SceneComponent.K2_SetWorldRotation` _springarm (`KismetMathLibrary.MakeRotator` 0.0 Pitch Yaw) false false))

(fn `Adjust the scale`
  (params (Scale :type "Float (double-precision)"))
  (`self.SetActorScale3D` (`KismetMathLibrary.MakeVector` Scale Scale Scale)))

(fn `UserConstructionScript`)